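; LibraryCube is a destructible library structure with health that shatters when that health runs out.
; On BeginPlay it creates a LibraryBar health widget, passing itself, its max health and a bar height, and adds it to the viewport.
; Tick polls Health and, once at zero or below, enables physics, applies destructible damage at the center of mass and removes the bar, guarded by a Destroyed flag.
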(event EventBeginPlay
  ;[1 1 1] Add widget to cube
  (bind _returnvalue (UserInterface|CreateWidget "/Game/FEUPDEFENSE/Widget/LibraryBar.LibraryBar_C" 0 (Variables|Default|GetMAX_HEALTH) self (Variables|Default|GetHealth%20Bar%20Height)))
  (bind _output_get (Variables|Default|SetHealth%20Bar _returnvalue))
  (UserInterface|Viewport|AddtoViewport _output_get 0))

(event EventTick
  (params (DeltaSeconds :type Float%20%28single-precision%29))
  ;[1 1 1] When library reaches 0 health it explodes
  (if (not (Variables|Default|GetDestroyed))
    (if (<= (Variables|Default|GetHealth) 0)
      (Variables|Default|SetDestroyed true)
      (Physics|SetSimulatePhysics true)
      (bind _returnvalue (Physics|GetCenterOfMass "None"))
      (Game|Damage|ApplyDamage 2.0 _returnvalue _returnvalue 5.0)
      (Widget|RemovefromParent (Variables|Default|GetHealth%20Bar)))))

(event EventActorBeginOverlap
  (params (OtherActor :type Actor%20Object%20Reference)))

(fn ConstructionScript)
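; Clickable tower-defense turret that the player powers on or off against the camera pawn's shared energy budget.
; When energy is short, powering on switches off another active turret instead.
; Each tick it yaws smoothly toward the current visible MovingCube in range, advancing the target index past hidden ones.
; While powered, it spawns socket projectiles throttled by a Delay, regardless of target range.
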(event OnClicked(simple_turret)
  (params (TouchedComponent :type Primitive%20Component%20Object%20Reference))
  (if (Variables|Default|GetStatus)
    (Variables|Default|SetStatus false)
    (Variables|/Game/FEUPDEFENSE/Blueprints/Controller/td_camera.td_camera_C|SetCurrentEnergy (stale _astd_camera) (- (Variables|/Game/FEUPDEFENSE/Blueprints/Controller/td_camera.td_camera_C|GetCurrentEnergy (stale _astd_camera)) (Variables|Default|GetEnergy)))
    (else
      (bind _astd_camera (Utilities|Casting|CastTotd_camera (Game|Player|GetPlayerPawn 0)))
      (if (< (+ (Variables|/Game/FEUPDEFENSE/Blueprints/Controller/td_camera.td_camera_C|GetCurrentEnergy _astd_camera) (Variables|Default|GetEnergy)) (Variables|/Game/FEUPDEFENSE/Blueprints/Controller/td_camera.td_camera_C|GetTotalEnergy _astd_camera))
        (Variables|/Game/FEUPDEFENSE/Blueprints/Controller/td_camera.td_camera_C|SetCurrentEnergy _astd_camera (+ (Variables|/Game/FEUPDEFENSE/Blueprints/Controller/td_camera.td_camera_C|GetCurrentEnergy _astd_camera) (Variables|Default|GetEnergy)))
        (Variables|Default|SetStatus true)
        (else
          (bind _outactors (Actor|GetAllActorsOfClass "turret_blueprint_C"))
          (bind _array_element (Utilities|Array|ForEachLoopwithBreak _outactors :!label _label)
            (:LoopBody
              (if (Variables|turret_blueprint_C|GetStatus _array_element)
                (Variables|turret_blueprint_C|SetStatus _array_element false)
                (Variables|Default|SetStatus true)
                (goto _label Break)))))))))

(event OnBeginCursorOver(simple_turret)
  (params (TouchedComponent :type Primitive%20Component%20Object%20Reference))
  ;[1 1 1] Change Cursor
  (Variables|/Script/Engine.PlayerController|SetCurrentMouseCursor (Game|GetPlayerController 0) "Hand"))

(event OnEndCursorOver(simple_turret)
  (params (TouchedComponent :type Primitive%20Component%20Object%20Reference))
  ;[1 1 1] Change Cursor
  (Variables|/Script/Engine.PlayerController|SetCurrentMouseCursor (Game|GetPlayerController 0) "Default"))

(event Custom|SelectTarget
  ;[1 1 1] Find and Kill
  (bind _outactors (Actor|GetAllActorsOfClass "/Game/FEUPDEFENSE/Blueprints/MovingCube.MovingCube_C"))
  (if (!= (Utilities|Array|Length _outactors) 0)
    (if (Rendering|IsVisible (Utilities|Array|Get(acopy) _outactors (Variables|Default|GetCurrentEny)))
      (if (< (Transformation|GetDistanceTo (Utilities|Array|Get(acopy) _outactors (Variables|Default|GetCurrentEny)) self) (Variables|TurretSettings|GetAttackRange))
        (Transformation|SetWorldRotation (Variables|Default|Getsimple_turret) (Math|Interpolation|RInterpTo (Transformation|GetWorldRotation (Variables|Default|Getsimple_turret)) (Class|KismetMathLibrary|MakeRot 0.0 (.Yaw (Class|KismetMathLibrary|BreakRot (Math|Rotator|FindLookatRotation (Transformation|GetWorldLocation (Variables|Default|Getsimple_turret)) (Transformation|GetActorLocation (Utilities|Array|Get(acopy) _outactors (Variables|Default|GetCurrentEny)))))) 0.0) (Variables|Default|GetDeltaTime) (Variables|TurretSettings|GetRotationSpeed)) false))
      (elif (< (+ (Variables|Default|GetCurrentEny) 1) (Utilities|Array|Length _outactors))
        (Variables|Default|SetCurrentEny (+ (Variables|Default|GetCurrentEny) 1))))))

(event Custom|FireWeapons
  ;[1 1 1] Fire Weapons
  (Utilities|FlowControl|Delay (Variables|TurretSettings|GetFireInterval))
  (bind _returnvalue (Game|SpawnActorfromClass "/Game/Turret/Projectile.Projectile_C" (Transformation|GetSocketTransform (Variables|Default|Getsimple_turret) (Utilities|Array|Get(acopy) (Transformation|GetAllSocketNames)) "RTS_World") false 0))
  (Transformation|SetActorScale3D _returnvalue "1.000000,1.000000,1.000000"))

(event EventTick
  (params (DeltaSeconds :type Float%20%28single-precision%29))
  ;[1 1 1] Game Sequence
  (Variables|Default|SetDeltaTime DeltaSeconds)
  (CallFunction|SelectTarget)
  (if (Variables|Default|GetStatus)
    (CallFunction|FireWeapons)))

(event EventBeginPlay
  ;[1 1 1] Change Cursor
  (Variables|/Script/Engine.PlayerController|SetbEnableMouseOverEvents (Game|GetPlayerController 0) true))

(fn ConstructionScript)
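; MovingCube is an actor with health that can be shot by projectiles and damages the library when it reaches a trigger box.
; On BeginPlay it creates a viewport HealthBar widget linked to itself, removed when the actor is destroyed.
; Projectile hits on the cube or capsule share one damage path, which at zero health destroys components and hides visuals rather than destroying the actor.
; Overlapping the trigger reduces the first LibraryCube's health and destroys the actor.
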(event OnComponentBeginOverlap(Cube)
  (params (OtherActor :type Actor%20Object%20Reference) (OtherComp :type Primitive%20Component%20Object%20Reference) (OtherBodyIndex :type Integer) (bFromSweep :type Boolean) (SweepResult :type Hit%20Result%20Structure%20%28by%20ref%29))
  ;[1 1 1] Destroy itself and damage the library on colision
  (if (== (Utilities|GetClass OtherActor) "/Game/FEUPDEFENSE/Blueprints/TriggerBox_Blueprint.TriggerBox_Blueprint_C")
    (bind _outactors (Actor|GetAllActorsOfClass "/Game/FEUPDEFENSE/Blueprints/LibraryCube_DM_Blueprint.LibraryCube_DM_Blueprint_C"))
    (Variables|/Game/FEUPDEFENSE/Blueprints/LibraryCube_DM_Blueprint.LibraryCube_DM_Blueprint_C|SetHealth (Utilities|Array|Get(acopy) _outactors) (- (Variables|/Game/FEUPDEFENSE/Blueprints/LibraryCube_DM_Blueprint.LibraryCube_DM_Blueprint_C|GetHealth (Utilities|Array|Get(acopy) _outactors)) 10))
    (Actor|DestroyActor)))

(event OnComponentHit(CapsuleComponent)
  (params (OtherActor :type Actor%20Object%20Reference) (OtherComp :type Primitive%20Component%20Object%20Reference) (NormalImpulse :type Vector :default "0, 0, 0") (Hit :type Hit%20Result%20Structure%20%28by%20ref%29))
  ;[1 1 1] Destroy cube once colided with a projectile
  (if (== (Utilities|GetClass OtherActor) "/Game/Turret/Projectile.Projectile_C")
    (bind _output_get (Variables|Default|Sethealth (- (Variables|Default|Gethealth) 1)))
    (if (== _output_get 0)
      (Components|DestroyComponent)
      (Components|DestroyComponent)
      (Variables|Default|SetbAutoDestroyWhenFinished true)
      (Rendering|SetVisibility false false))))

(event OnComponentHit(Cube)
  (params (OtherActor :type Actor%20Object%20Reference) (OtherComp :type Primitive%20Component%20Object%20Reference) (NormalImpulse :type Vector :default "0, 0, 0") (Hit :type Hit%20Result%20Structure%20%28by%20ref%29))
  ;[1 1 1] Destroy cube once colided with a projectile
  (if (== (Utilities|GetClass OtherActor) "/Game/Turret/Projectile.Projectile_C")
    (bind _output_get (Variables|Default|Sethealth (- (Variables|Default|Gethealth) 1)))
    (if (== _output_get 0)
      (Components|DestroyComponent)
      (Components|DestroyComponent)
      (Variables|Default|SetbAutoDestroyWhenFinished true)
      (Rendering|SetVisibility false false))))

(event EventDestroyed
  ;[1 1 1] Add widget to cube
  (Widget|RemovefromParent (Variables|Default|GetHealthBar)))

(event EventBeginPlay
  ;[1 1 1] Add widget to cube
  (bind _returnvalue (UserInterface|CreateWidget "/Game/FEUPDEFENSE/Widget/HealthBar.HealthBar_C" 0 (Variables|Default|GetMAX_HEALTH) self (Variables|Default|GetHealth%20Bar%20Height)))
  (bind _output_get (Variables|Default|SetHealthBar _returnvalue))
  (UserInterface|Viewport|AddtoViewport _returnvalue 0))

(fn ConstructionScript)